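; Player controller for a Minesweeper game that manages the HUD, option menu and game-over screen.
; BeginPlay creates the game widget and a paused one-second minute/second timer, then opens the options widget, which also reopens on OptionMenu input.
; Tick refreshes timer and flag text from the GameMode's grid, and shows points and time on game over.
; Both menus pause the game and disable click, hover and touch events.
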(event EventTick
  (params (DeltaSeconds :type Float%20%28single-precision%29))
  (bind _self self)
  (bind _bp_gamemode (Variables|Default|GetBP_GameMode))
  (Rendering|Components|TextRender|SetText (Variables|/Game/Blueprint/Widgets/WBP_GameWidget.WBP_GameWidget_C|GetTextBlockTimer (Variables|Default|GetGameWidget)) (Utilities|Text|ToText(String) (Utilities|String|Append (Utilities|String|ToString(Text) (Utilities|Text|ToText(Integer) (Variables|Default|GetMinutes) false true 2)) ":" (Utilities|String|ToString(Text) (Utilities|Text|ToText(Integer) (Variables|Default|GetSeconds) false true 2)))))
  (bind _returnvalue (Class|GridActor|GetHowManyFlags (Variables|/Script/MineSweeper.MineSweeperGameModeBase|GetGridActor (Variables|Default|GetBP_GameMode))))
  (Rendering|Components|TextRender|SetText (Variables|/Game/Blueprint/Widgets/WBP_GameWidget.WBP_GameWidget_C|GetTextBlockFlags (Variables|Default|GetGameWidget)) (Utilities|Text|ToText(String) (Utilities|String|Append "Flags: " (Utilities|String|ToString(Integer) _returnvalue))))
  (if (Variables|/Script/MineSweeper.MineSweeperGameModeBase|GetGameOver _bp_gamemode)
    (Variables|/Script/MineSweeper.MineSweeperGameModeBase|SetGameOver _bp_gamemode false)
    (bind _returnvalue_2 (UserInterface|CreateWidget "/Game/Blueprint/Widgets/WBP_GameOver.WBP_GameOver_C" (Game|GetPlayerController 0)))
    (UserInterface|Viewport|AddtoViewport _returnvalue_2 0)
    (Rendering|Components|TextRender|SetText (Variables|/Game/Blueprint/Widgets/WBP_GameOver.WBP_GameOver_C|GetTextBlock_Points _returnvalue_2) (Utilities|Text|ToText(Integer) (Variables|/Script/MineSweeper.MineSweeperGameModeBase|GetTotalPoints (Variables|Default|GetBP_GameMode))))
    (Rendering|Components|TextRender|SetText (Variables|/Game/Blueprint/Widgets/WBP_GameOver.WBP_GameOver_C|GetTextBlock_Time _returnvalue_2) (Utilities|Text|ToText(String) (Utilities|String|Append (Utilities|String|ToString(Text) (Utilities|Text|ToText(Integer) (Variables|Default|GetMinutes) false true 2)) ":" (Utilities|String|ToString(Text) (Utilities|Text|ToText(Integer) (Variables|Default|GetSeconds) false true 2)))))
    (Game|SetGamePaused true)
    (Variables|Default|SetbEnableClickEvents _self false)
    (Variables|Default|SetbEnableMouseOverEvents _self false)
    (Variables|Default|SetbEnableTouchEvents _self false)
    (Variables|Default|SetbEnableTouchOverEvents _self false)))

(event EventBeginPlay
  (bind _self self)
  (bind _returnvalue (UserInterface|CreateWidget "/Game/Blueprint/Widgets/WBP_GameWidget.WBP_GameWidget_C" (Game|GetPlayerController 0)))
  (bind _output_get (Variables|Default|SetGameWidget _returnvalue))
  (UserInterface|Viewport|AddtoViewport _output_get 0)
  (bind _returnvalue_2 (Utilities|Time|SetTimerbyFunctionName 0 "Timer" 1.0 true))
  (bind _output_get_2 (Variables|Default|SetTimeHandle _returnvalue_2))
  (Utilities|Time|PauseTimerbyHandle _output_get_2)
  (bind _asbp_mine_sweeper_game_mode_base (Utilities|Casting|CastToBP_MineSweeperGameModeBase (Game|GetGameMode)))
  (Variables|Default|SetBP_GameMode _asbp_mine_sweeper_game_mode_base)
  (bind _returnvalue_3 (UserInterface|CreateWidget "/Game/Blueprint/Widgets/WBP_OptionWidget.WBP_OptionWidget_C" (Game|GetPlayerController 0)))
  (UserInterface|Viewport|AddtoViewport _returnvalue_3 0)
  (Game|SetGamePaused true)
  (Variables|Default|SetbEnableClickEvents _self false)
  (Variables|Default|SetbEnableMouseOverEvents _self false)
  (Variables|Default|SetbEnableTouchEvents _self false)
  (Variables|Default|SetbEnableTouchOverEvents _self false))

(event Input|ActionEvents|InputActionOptionMenu
  (params (Key :type Key%20Structure :default "None"))
  (bind _self self)
  (:Pressed
    (bind _returnvalue (UserInterface|CreateWidget "/Game/Blueprint/Widgets/WBP_OptionWidget.WBP_OptionWidget_C" (Game|GetPlayerController 0)))
    (UserInterface|Viewport|AddtoViewport _returnvalue 0)
    (Game|SetGamePaused true)
    (Variables|Default|SetbEnableClickEvents _self false)
    (Variables|Default|SetbEnableMouseOverEvents _self false)
    (Variables|Default|SetbEnableTouchEvents _self false)
    (Variables|Default|SetbEnableTouchOverEvents _self false)))

(fn ConstructionScript)

(fn Timer
  (Math|Integer|IncrementInt (Variables|Default|GetSeconds)
    (:%20%20
      (if (== (Variables|Default|GetSeconds) 60)
        (Variables|Default|SetSeconds 0)
        (Math|Integer|IncrementInt (Variables|Default|GetMinutes))))))